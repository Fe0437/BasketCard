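; BasketGenerator is an actor that spawns a row of Basket actors across the width of its Box, each assigned an Emotion.
; The CreateBaskets event centers each basket in an equal slice of the box's X extent and cycles through AvailableEmotions by index modulo.
; Baskets spawn at origin-centered offsets, then attach to the generator with KeepRelative, so those offsets become local to it.
; Nothing in this graph calls CreateBaskets.
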(event Custom|Create%20Baskets
  (bind _numberofbaskets (Variables|Default|GetnumberOfBaskets))
  (bind _box (Variables|Default|GetBox))
  (bind _availableemotions (Variables|Default|GetAvailableEmotions))
  (bind _returnvalue (Math|Conversions|ToFloat(Integer) _numberofbaskets))
  (bind _boxextent (Variables|/Script/Engine.BoxComponent|GetBoxExtent _box))
  (bind _x (Math|Vector|BreakVector _boxextent))
  (bind _returnvalue_2 (* _x 2.0))
  (bind _returnvalue_3 (/ _returnvalue_2 _returnvalue))
  (for _index (range 0 _numberofbaskets)
    (bind _returnvalue_4 (Game|SpawnActorfromClass "/Game/CardBasket/Blueprints/Basket.Basket_C" (Math|Conversions|ToTransform(Vector) (+ (Math|Vector|MakeVector (+ (* _returnvalue_3 (Math|Conversions|ToFloat(Integer) _index)) (* _returnvalue_3 0.5)) 0.0 0.0) (- "0, 0, 0" (Math|Vector|MakeVector _x 0.0 0.0)))) "AlwaysSpawn" 0 (Utilities|Array|Get(acopy) _availableemotions (Math|Integer|%(Integer) _index (Utilities|Array|Length _availableemotions))) 0))
    (Transformation|AttachActorToActor _returnvalue_4 self "None" "KeepRelative" "KeepRelative" "KeepRelative" true)))

(event EventBeginPlay)

(event Collision|EventActorBeginOverlap
  (params (OtherActor :type Actor%20Object%20Reference)))

(event EventTick
  (params (DeltaSeconds :type Float%20%28single-precision%29)))

(fn ConstructionScript)